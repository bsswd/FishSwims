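; BP_CloseupForeground is an environment actor that scrolls along its forward axis, apparently as moving foreground scenery.
; It begins moving one second after BeginPlay, with StartMoving and StopMoving events toggling motion and Reverse flip-flopping the direction.
; Tick offsets its location by forward vector, signed Speed and DeltaSeconds without sweeping, travelling backward unless reversed and applying zero speed when stopped.
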(event EventBeginPlay
  (Utilities|FlowControl|Delay 1.0)
  (Variables|Controls|SetIsMoving true))

(event EventReverse
  (Utilities|FlowControl|FlipFlop
    (:A
      (Variables|Controls|SetIsReverse true))
    (:B
      (Variables|Controls|SetIsReverse false))))

(event EventStopMoving
  (Variables|Controls|SetIsMoving false))

(event EventTick
  (params (DeltaSeconds :type Float%20%28single-precision%29))
  (if (Variables|Controls|GetIsReverse)
    (Variables|Controls|SetDirection 1.0)
    (else
      (Variables|Controls|SetDirection -1.0)))
  (if (Variables|Controls|GetIsMoving)
    (Transformation|SetActorLocation (CallFunction|CalculateNewLocation (* (Variables|Controls|GetSpeed) (Variables|Controls|GetDirection)) DeltaSeconds) false false)
    (else
      (Transformation|SetActorLocation (CallFunction|CalculateNewLocation 0.0 DeltaSeconds) false false))))

(event EventStartMoving
  (Variables|Controls|SetIsMoving true))

(fn ConstructionScript)

(fn CalculateNewLocation
  (params (Speed :type Float%20%28double-precision%29) (DeltaSeconds :type Float%20%28double-precision%29))
  (return (+ (Transformation|GetActorLocation) (* (* (Transformation|GetActorForwardVector) Speed) DeltaSeconds))))