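; BP_BasePlant is a base Blueprint for environment plants animated with Spine.
; On BeginPlay it copies its Animation (atlas) and Skeleton (data) variables into the SpineSkeleton and SpineSkeletonAnimation components, then loops the track named "animation".
; The construction script only calls its parent, so this Blueprint assigns those assets at runtime.
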(event EventBeginPlay
  (bind _spineskeletonanimation (Variables|Default|GetSpineSkeletonAnimation))
  (bind _spineskeleton (Variables|Default|GetSpineSkeleton))
  (|CallParentFunction)
  (Variables|/Script/SpinePlugin.SpineSkeletonComponent|SetAtlas _spineskeleton (Variables|Default|GetAnimation))
  (Variables|/Script/SpinePlugin.SpineSkeletonComponent|SetSkeletonData _spineskeleton (Variables|Default|GetSkeleton))
  (Variables|/Script/SpinePlugin.SpineSkeletonComponent|SetAtlas _spineskeletonanimation (Variables|Default|GetAnimation))
  (Variables|/Script/SpinePlugin.SpineSkeletonComponent|SetSkeletonData _spineskeletonanimation (Variables|Default|GetSkeleton))
  (Class|SpineSkeletonAnimationComponent|SetAnimation (Variables|Default|GetSpineSkeletonAnimation) 0 "animation" true))

(fn ConstructionScript
  (|CallParentFunction))