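; Countdown spawner actor that releases NPCs while a timer runs and spawns a single BP_Grandpa when it expires.
; Tick feeds a one-second Delay into a Timer macro, whose updates drive a delayed loop spawning random neutral NPCs near SpawnLoc with random height offsets.
; Both SpawnEnemy branches reach that neutral loop; the enemy-wave loop is disconnected.
; SpawnNpc returns inside its loop, and SpawnNpcAtTime is uncalled.
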(event EventTick
  (params (DeltaSeconds :type Float%20%28single-precision%29))
  (bind _spawnloc (Variables|Default|GetSpawnLoc))
  (bind _returnvalue (Transformation|GetWorldLocation _spawnloc))
  (Utilities|FlowControl|Delay 1.0)
  (Utilities|Timer (Variables|Timer|GetMinutes) (Variables|Timer|GetSeconds)
    (:Complete
      ;[0 1 0.06418] Spawn Grandpa
      (Utilities|FlowControl|DoOnce false
        (:Completed
          (CallFunction|SpawnNpc "/Game/Characters/NPC/Friend/BP_Grandpa.BP_Grandpa_C" 1 (Transformation|GetWorldLocation (Variables|Default|GetSpawnLoc)) 0.0)
          (Variables|Default|SetSpawnEnemy? false))))
    (:Update
      (if (Variables|Default|GetSpawnEnemy?)
        (Utilities|FlowControl|Sequence
          (:then_1
            _)))
      ;[1 0.9449 0.01481] Spawn neutrals from period
      (for _index (range 0 15)
        (Utilities|FlowControl|Delay 5.0)
        (CallFunction|SpawnNpc (.OutItem (Utilities|Array|Random (Variables|NPC|GetNeutralToSpawn))) (Math|Random|RandomIntegerinRange 1 1) (Math|Vector|MakeVector (.x _returnvalue) (- (.y _returnvalue) 8e+01) (.z _returnvalue)) (Math|Random|RandomFloatinRange -5e+01 8e+01))))))

(fn ConstructionScript)

(fn SpawnNpcatTime
  (params (Npc :type BP%20NPC%20Class%20Reference) (Minutes :type Integer) (Seconds :type Integer) (Quantity :type Integer) (Location :type Vector) (ZOfset :type Float%20%28double-precision%29))
  (LocalVariables|SetSpawnLocation Location)
  (if (and (== (Variables|Timer|GetMinutes) Minutes) (== (Variables|Timer|GetSeconds) Seconds))
    (for _index (range 1 Quantity)
      (Game|SpawnActorfromClass Npc (Math|Transform|MakeTransform (Math|Vector|MakeVector (.x (LocalVariables|GetSpawnLocation)) (.y (LocalVariables|GetSpawnLocation)) (+ (.z (LocalVariables|GetSpawnLocation)) ZOfset)) "0, 0, 0" "1.000000,1.000000,1.000000") "Undefined" "MultiplyWithRoot" 0 0))))

(fn SpawnNpc
  (params (Npc :type BP%20NPC%20Class%20Reference) (Quantity :type Integer) (Location :type Vector) (ZOfset :type Float%20%28double-precision%29))
  (LocalVariables|SetSpawnLocation Location)
  (for _index (range 1 Quantity)
    (bind _returnvalue (Game|SpawnActorfromClass Npc (Math|Transform|MakeTransform (Math|Vector|MakeVector (.x (LocalVariables|GetSpawnLocation)) (.y (LocalVariables|GetSpawnLocation)) (+ (.z (LocalVariables|GetSpawnLocation)) ZOfset)) "0, 0, 0" "1.000000,1.000000,1.000000") "Undefined" "MultiplyWithRoot" 0 0))
    (return _returnvalue)))