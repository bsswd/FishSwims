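; BP_Timer is a countdown actor that spawns NPCs at the player fish's spawn point.
; A one-second Delay on Tick drives a Timer macro that decrements Minutes and Seconds.
; Each update calls SpawnNpcAtTime to spawn a group of dolphins at a set time, while reaching zero spawns Grandpa, repeating every second thereafter.
; A random enemy wave loop is present but disconnected.
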(event EventTick
  (params (DeltaSeconds :type Float%20%28single-precision%29))
  (bind _player (Variables|Default|GetPlayer))
  (bind _spawnpoint (Variables|/Game/Characters/BP_Fish.BP_Fish_C|GetSpawnPoint _player))
  (bind _returnvalue (Transformation|GetWorldLocation _spawnpoint))
  (Utilities|FlowControl|Delay 1.0)
  (Utilities|Timer (Variables|Default|GetMinutes) (Variables|Default|GetSeconds)
    (:Complete
      ;[1 1 1] Spawn Grandpa
      (CallFunction|SpawnNpc "/Game/Characters/NPC/Friend/BP_Grandpa.BP_Grandpa_C" 1 _returnvalue 0.0))
    (:Update
      (Utilities|IsValid _player
        (:Is%20Valid
          (CallFunction|SpawnNpcatTime "/Game/Characters/NPC/Enemy/BP_Dolphin.BP_Dolphin_C" 1 59 5 _returnvalue 0.0))))))

(event EventBeginPlay
  (bind _asbp_fish (Utilities|Casting|CastToBP_Fish (Game|Player|GetPlayerPawn 0)))
  (Variables|Default|SetPlayer _asbp_fish))

(fn ConstructionScript)

(fn SpawnNpcatTime
  (params (Npc :type BP%20NPC%20Class%20Reference) (Minutes :type Integer) (Seconds :type Integer) (Quantity :type Integer) (Location :type Vector) (ZOfset :type Float%20%28double-precision%29))
  (LocalVariables|SetSpawnLocation Location)
  (if (and (== (Variables|Default|GetMinutes) Minutes) (== (Variables|Default|GetSeconds) Seconds))
    (for _index (range 1 Quantity)
      (Game|SpawnActorfromClass Npc (Math|Transform|MakeTransform (Math|Vector|MakeVector (.x (LocalVariables|GetSpawnLocation)) (.y (LocalVariables|GetSpawnLocation)) (+ (.z (LocalVariables|GetSpawnLocation)) ZOfset)) "0, 0, 0" "1.000000,1.000000,1.000000") "Undefined" "MultiplyWithRoot" 0 0))))

(fn SpawnNpc
  (params (Npc :type BP%20NPC%20Class%20Reference) (Quantity :type Integer) (Location :type Vector) (ZOfset :type Float%20%28double-precision%29))
  (LocalVariables|SetSpawnLocation Location)
  (for _index (range 1 Quantity)
    (Game|SpawnActorfromClass Npc (Math|Transform|MakeTransform (Math|Vector|MakeVector (.x (LocalVariables|GetSpawnLocation)) (.y (LocalVariables|GetSpawnLocation)) (+ (.z (LocalVariables|GetSpawnLocation)) ZOfset)) "0, 0, 0" "1.000000,1.000000,1.000000") "Undefined" "MultiplyWithRoot" 0 0)))