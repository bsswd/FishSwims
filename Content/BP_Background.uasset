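; BP_Background is an actor that scrolls itself backward along its own forward axis at a set Speed, likely as a moving background.
; It starts moving one second after BeginPlay, and StartMoving and StopMoving events toggle the IsMoving flag.
; Each Tick sets its location through CalculateNewLocation, a frame-rate-independent offset from the forward vector, passing zero speed while stopped.
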(event EventBeginPlay
  (Utilities|FlowControl|Delay 1.0)
  (Variables|Default|SetIsMoving true))

(event EventStopMoving
  (Variables|Default|SetIsMoving false))

(event EventTick
  (params (DeltaSeconds :type Float%20%28single-precision%29))
  (if (Variables|Default|GetIsMoving)
    (Transformation|SetActorLocation (CallFunction|CalculateNewLocation (* (Variables|Default|GetSpeed) -1.0) DeltaSeconds) false false)
    (else
      (Transformation|SetActorLocation (CallFunction|CalculateNewLocation 0.0 DeltaSeconds) false false))))

(event EventStartMoving
  (Variables|Default|SetIsMoving true))

(fn ConstructionScript)

(fn CalculateNewLocation
  (params (Speed :type Float%20%28double-precision%29) (DeltaSeconds :type Float%20%28double-precision%29))
  (return (+ (Transformation|GetActorLocation) (* (* (Transformation|GetActorForwardVector) Speed) DeltaSeconds))))