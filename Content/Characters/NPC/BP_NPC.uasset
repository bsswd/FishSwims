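; NPC base logic that sets up movement stats when the character spawns.
; BeginPlay calls the parent, then InitNpcStats, which randomizes Speed within a given range, stores DirectionX and picks a random DirectionZ between down and up.
; BeginPlay passes zero for every input, so only DirectionZ varies here.
; Nothing in this Blueprint applies these values to movement, and Tick is disabled.
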(event EventBeginPlay
  (|CallParentFunction)
  (CallFunction|InitNpcStats 0.0 0.0 0.0))

(event Collision|EventActorBeginOverlap
  (params (OtherActor :type Actor%20Object%20Reference))
  (|CallParentFunction OtherActor) ; This node is disabled and will not be called.\nDrag off pins to build functionality.
)

(event EventTick
  (params (DeltaSeconds :type Float%20%28single-precision%29))
  (|CallParentFunction DeltaSeconds) ; This node is disabled and will not be called.\nDrag off pins to build functionality.
)

(fn ConstructionScript
  (|CallParentFunction))

(fn InitNpcStats
  (params (MinSpeed :type Float%20%28double-precision%29) (MaxSpeed :type Float%20%28double-precision%29) (DirectionX :type Float%20%28double-precision%29))
  (Variables|Default|SetSpeed (Math|Random|RandomFloatinRange MinSpeed MaxSpeed))
  (Variables|Default|SetDirectionX DirectionX)
  (Variables|Default|SetDirectionZ (Math|Random|RandomFloatinRange -1.0 1.0)))