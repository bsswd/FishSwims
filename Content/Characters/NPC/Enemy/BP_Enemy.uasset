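; BP_Enemy is an NPC enemy that moves across the screen on X and Z and destroys itself past the horizontal bounds.
; It initializes stats through inherited NPC logic, loops a Spine animation and applies movement each tick.
; Events steer it: fish impact sets upward Z, ChangeZdirection inverts Z, and a ball hit reverses X, randomizes Z, flips it and plays a random-pitch sound with a brief red tint.
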(event EventBeginPlay
  (|CallParentFunction)
  (CallFunction|InitNpcStats 0.0 0.0 -1.0)
  ;[1 1 1] Set animation
  (Class|SpineSkeletonAnimationComponent|SetAnimation (Variables|Default|GetSpineSkeletonAnimation) 0 "animation" true))

(event Collision|EventActorBeginOverlap
  (params (OtherActor :type Actor%20Object%20Reference))
  (|CallParentFunction OtherActor))

(event EventTick
  (params (DeltaSeconds :type Float%20%28single-precision%29))
  (bind _returnvalue (Transformation|GetActorLocation))
  (|CallParentFunction DeltaSeconds)
  (CallFunction|Movement false (Variables|Default|GetDirectionX) (Variables|Default|GetDirectionZ) (Variables|Default|GetSpeed) DeltaSeconds)
  ;[1 1 1] Destroy after leaving screen
  (if (or (< (.x _returnvalue) -1e+03) (> (.x _returnvalue) 1e+03))
    (Actor|DestroyActor)))

(event EventInteract
  ;[1 1 1] Impact to fish
  (Variables|Default|SetDirectionZ 1.0))

(event EventHitBall
  (bind _spineskeletonrenderer (Variables|Default|GetSpineSkeletonRenderer))
  ;[1 1 1] Ball hit
  (CallFunction|Flip)
  (Audio|PlaySound2D "/Game/Sound/SC_HitEnemy.SC_HitEnemy" 1.0 (Math|Random|RandomFloatinRange 0.2 1.2) 0.0 0 0)
  (Variables|Default|SetDirectionX (* (Variables|Default|GetDirectionX) -1.0))
  (Variables|Default|SetDirectionZ (Math|Random|RandomFloatinRange -1.0 1.0))
  (Variables|/Script/SpinePlugin.SpineSkeletonRendererComponent|SetColor _spineskeletonrenderer "(R=0.786458,G=0.031713,B=0.000000,A=0.822000)")
  (Utilities|FlowControl|Delay 0.2)
  (Variables|/Script/SpinePlugin.SpineSkeletonRendererComponent|SetColor _spineskeletonrenderer "(R=1.000000,G=1.000000,B=1.000000,A=1.000000)"))

(event EventChangeZdirection
  ;[1 1 1] Change Z direction
  (Variables|Default|SetDirectionZ (* (Variables|Default|GetDirectionZ) -1.0)))

(fn ConstructionScript
  (|CallParentFunction))