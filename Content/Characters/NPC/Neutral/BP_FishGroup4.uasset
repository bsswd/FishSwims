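; BP_FishGroup4 is a neutral NPC fish group that moves along one axis in the negative direction.
; BeginPlay picks a random speed within a fixed range, and Tick passes it with the fixed direction and delta time to a Movement function defined outside this graph.
; Begin play, overlap, tick and construction all call their parent implementations, with overlap and construction adding no logic of their own.
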(event EventBeginPlay
  (|CallParentFunction)
  (Variables|Default|SetSpeed (Math|Random|RandomFloatinRange 5e+01 9e+01)))

(event Collision|EventActorBeginOverlap
  (params (OtherActor :type Actor%20Object%20Reference))
  (|CallParentFunction OtherActor))

(event EventTick
  (params (DeltaSeconds :type Float%20%28single-precision%29))
  (|CallParentFunction DeltaSeconds)
  (CallFunction|Movement false -1.0 0.0 (Variables|Default|GetSpeed) DeltaSeconds))

(fn ConstructionScript
  (|CallParentFunction))