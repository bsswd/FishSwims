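; BP_AFishGroup is a neutral NPC fish group that drifts along negative X at constant speed, with a randomized Spine appearance.
; On BeginPlay it draws atlas and skeleton data from random Asset entries and applies them to both Spine components.
; Atlas and data come from separate Random evaluations, so they can come from different entries.
; Tick calls Movement each frame; overlap and construction only defer to the parent.
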(event EventBeginPlay
  (bind _spineskeletonanimation (Variables|Default|GetSpineSkeletonAnimation))
  (bind _asset (Variables|Default|GetAsset))
  (bind _spineskeleton (Variables|Default|GetSpineSkeleton))
  (bind _outitem (Utilities|Array|Random _asset))
  (|CallParentFunction)
  (Variables|Default|SetNewAtlas (.atlas _outitem))
  (Variables|Default|SetNewData (.data _outitem))
  (Variables|/Script/SpinePlugin.SpineSkeletonComponent|SetAtlas _spineskeleton (Variables|Default|GetNewAtlas))
  (Variables|/Script/SpinePlugin.SpineSkeletonComponent|SetSkeletonData _spineskeleton (Variables|Default|GetNewData))
  (Variables|/Script/SpinePlugin.SpineSkeletonComponent|SetAtlas _spineskeletonanimation (Variables|Default|GetNewAtlas))
  (Variables|/Script/SpinePlugin.SpineSkeletonComponent|SetSkeletonData _spineskeletonanimation (Variables|Default|GetNewData)))

(event Collision|EventActorBeginOverlap
  (params (OtherActor :type Actor%20Object%20Reference))
  (|CallParentFunction OtherActor))

(event EventTick
  (params (DeltaSeconds :type Float%20%28single-precision%29))
  (|CallParentFunction DeltaSeconds)
  (CallFunction|Movement false -1.0 0.0 5e+01 DeltaSeconds))

(fn ConstructionScript
  (|CallParentFunction))