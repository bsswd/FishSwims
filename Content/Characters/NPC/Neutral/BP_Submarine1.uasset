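; BP_Submarine1 is a neutral NPC submarine that moves steadily along the negative X direction.
; BeginPlay picks a random speed, and Tick passes it with a fixed direction and delta time to a Movement function not defined in this graph.
; The overlap event is disabled, and the construction script only calls its parent.
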(event EventBeginPlay
  (|CallParentFunction)
  (Variables|Default|SetSpeed (Math|Random|RandomFloatinRange 6e+01 1e+02)))

(event Collision|EventActorBeginOverlap
  (params (OtherActor :type Actor%20Object%20Reference))
  (|CallParentFunction OtherActor) ; This node is disabled and will not be called.\nDrag off pins to build functionality.
)

(event EventTick
  (params (DeltaSeconds :type Float%20%28single-precision%29))
  (|CallParentFunction DeltaSeconds)
  (CallFunction|Movement false -1.0 0.0 (Variables|Default|GetSpeed) DeltaSeconds))

(fn ConstructionScript
  (|CallParentFunction))