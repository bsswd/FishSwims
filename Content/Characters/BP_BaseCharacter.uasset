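; BP_BaseCharacter is a base character with a Spine skeleton animation, providing shared helpers for 2D movement and facing.
; Movement offsets the actor on the world X/Z plane by direction, speed and frame delta time unless Stop is set, bypassing movement-component logic.
; Flip mirrors the character by negating the Spine skeleton's X scale.
; The event graph and construction script are empty, so neither function is called here.
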(event EventBeginPlay)

(event Collision|EventActorBeginOverlap
  (params (OtherActor :type Actor%20Object%20Reference)))

(event EventTick
  (params (DeltaSeconds :type Float%20%28single-precision%29)))

(fn ConstructionScript)

(fn Movement
  (params (Stop :type Boolean) (DirectionX :type Float%20%28double-precision%29) (DirectionZ :type Float%20%28double-precision%29) (Speed :type Float%20%28double-precision%29))
  (bind _returnvalue (Utilities|Time|GetWorldDeltaSeconds))
  (bind _returnvalue_2 (* Speed _returnvalue))
  (if (not Stop)
    (Transformation|AddActorWorldOffset (Math|Vector|MakeVector (* DirectionX _returnvalue_2) 0.0 (* DirectionZ _returnvalue_2)))))

(fn Flip
  (bind _returnvalue (Class|SpineSkeletonComponent|GetScaleX (Variables|Default|GetSpineSkeletonAnimation)))
  (Class|SpineSkeletonComponent|SetScaleX (Variables|Default|GetSpineSkeletonAnimation) (* _returnvalue -1.0)))